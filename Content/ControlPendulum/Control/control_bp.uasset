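; Control board actor that lets the player operate a pendulum simulation with right-click.
; Three right-click handlers read ThirdPersonCharacter state to pick the action, with input enabled at BeginPlay.
; Planet selection sets PendulumRef's gravity for Earth, Mars or Moon and resets its swing, while length steps rescale the rod and update the readout.
; Two switches shift and recolour via material swaps, toggling the planet selection panel and equilibrium marker.
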(event `self.Box.OnComponentBeginOverlap`
  (params (OverlappedComponent :type "PrimitiveComponent Object Reference") (OtherActor :type "Actor Object Reference") (OtherComp :type "PrimitiveComponent Object Reference") (OtherBodyIndex :type Integer) (bFromSweep :type Boolean) (SweepResult :type "HitResult Structure (by ref)"))
  ;[1 1 1] Enable/Disable Input
)

(event `self.Box.OnComponentEndOverlap`
  (params (OverlappedComponent :type "PrimitiveComponent Object Reference") (OtherActor :type "Actor Object Reference") (OtherComp :type "PrimitiveComponent Object Reference") (OtherBodyIndex :type Integer))
  ;[1 1 1] Enable/Disable Input
)

(event `self.ReceiveBeginPlay`
  ;[1 1 1] Enable Input
  (`self.EnableInput` (`GameplayStatics.GetPlayerController` 0)))

(event `Key|RightMouseButton`
  (params (Key :type "Key Structure"))
  (bind _earthfinal (`self.EarthFinal`))
  (bind _moonfinal (`self.MoonFinal`))
  (bind _switchplanet (`self.SwitchPlanet`))
  (bind _switchplanet_2 (`self.SwitchPlanet`))
  (bind _pendulumref (`self.PendulumRef`))
  ;[1 1 1] Planet Switch
  (:`Pressed`
    (bind _asthird_person_character (cast `/Game/ThirdPersonBP/Blueprints/ThirdPersonCharacter` (`GameplayStatics.GetPlayerCharacter` 0)))
    (if (`/Game/ThirdPersonBP/Blueprints/ThirdPersonCharacter.SwitchOnPlanet` _asthird_person_character)
      (if (`self.CheckPlanetSwitchOn`)
        (`self.TurnOnOff` _switchplanet 2.0)
        (set `self.CheckPlanetSwitchOn` false)
        (`PrimitiveComponent.SetMaterial` _switchplanet_2 0 "/Game/ControlPendulum/Control/Materials/PlanetSwitchInstance_InstGreen.PlanetSwitchInstance_InstGreen")
        (`SceneComponent.ToggleVisibility` (`self.Selection_Box`) false)
        (`SceneComponent.ToggleVisibility` (`self.earthselect`) false)
        (`SceneComponent.ToggleVisibility` (`self.marsselect`) false)
        (`SceneComponent.ToggleVisibility` (`self.moonselect`) false)
        (`SceneComponent.ToggleVisibility` (`self.GlassPlate`) false)
        (else
          (`self.TurnOnOff` _switchplanet -2.0)
          (bind _output_get (set `self.CheckPlanetSwitchOn` true))
          (`PrimitiveComponent.SetMaterial` _switchplanet_2 0 "/Game/ControlPendulum/Control/Materials/PlanetSwitchInstance.PlanetSwitchInstance")
          (`SceneComponent.ToggleVisibility` (`self.Selection_Box`) false)
          (`SceneComponent.ToggleVisibility` (`self.earthselect`) false)
          (`SceneComponent.ToggleVisibility` (`self.marsselect`) false)
          (`SceneComponent.ToggleVisibility` (`self.moonselect`) false)
          (`SceneComponent.ToggleVisibility` (`self.GlassPlate`) false)))
      (elif _output_get
        (bind _earthmarsmoon (`/Game/ThirdPersonBP/Blueprints/ThirdPersonCharacter.EarthMarsMoon` _asthird_person_character))
        ;[1 1 1] MainBoardVisibilty
        (if (== _earthmarsmoon 0)
          (`SceneComponent.SetVisibility` _earthfinal true false)
          (`SceneComponent.SetVisibility` _moonfinal false false)
          (`SceneComponent.SetVisibility` (`self.Mars_Final`) false false)
          ;[1 1 1] Set Gravity
          (set `Pendulum.gravity` 981.0 _pendulumref)
          (set `Pendulum.angle` 0.785398 _pendulumref :!label _label)
          (set `Pendulum.angleA` 0.0 _pendulumref)
          (set `Pendulum.angleV` 0.0 _pendulumref)
          (elif (== _earthmarsmoon 1)
            (`SceneComponent.SetVisibility` (`self.Mars_Final`) true false)
            (`SceneComponent.SetVisibility` _earthfinal false false)
            (`SceneComponent.SetVisibility` _moonfinal false false)
            (set `Pendulum.gravity` 372.100006 _pendulumref)
            (goto _label)
            (elif (== _earthmarsmoon 2)
              (`SceneComponent.SetVisibility` _moonfinal true false)
              (`SceneComponent.SetVisibility` _earthfinal false false)
              (`SceneComponent.SetVisibility` (`self.Mars_Final`) false false)
              (set `Pendulum.gravity` 162.0 _pendulumref)
              (goto _label))))))))

(event `Key|RightMouseButton`
  (params (Key :type "Key Structure"))
  (bind _switchpendulum (`self.SwitchPendulum`))
  (:`Pressed`
    (bind _asthird_person_character (cast `/Game/ThirdPersonBP/Blueprints/ThirdPersonCharacter` (`GameplayStatics.GetPlayerCharacter` 0)))
    (if (`/Game/ThirdPersonBP/Blueprints/ThirdPersonCharacter.IsItOscillationSwitch` _asthird_person_character)
      (if (`/Game/ThirdPersonBP/Blueprints/ThirdPersonCharacter.IsSwitchOnForOscillation` _asthird_person_character)
        (set `/Game/ThirdPersonBP/Blueprints/ThirdPersonCharacter.IsSwitchOnForOscillation` false _asthird_person_character)
        (`PrimitiveComponent.SetMaterial` _switchpendulum 0 "/Game/ControlPendulum/Control/Materials/PlanetSwitchInstance_InstGreen.PlanetSwitchInstance_InstGreen")
        (`self.TurnOnOff` _switchpendulum 2.0)
        (else
          (set `/Game/ThirdPersonBP/Blueprints/ThirdPersonCharacter.IsSwitchOnForOscillation` true _asthird_person_character)
          (`PrimitiveComponent.SetMaterial` _switchpendulum 0 "/Game/ControlPendulum/Control/Materials/PlanetSwitchInstance.PlanetSwitchInstance")
          (`self.TurnOnOff` _switchpendulum -2.0)))
      (`SceneComponent.ToggleVisibility` (`/Game/Pendulum_bp/Pendulum_bp.EquilbriumPosition` (`self.PendulumRef`)) false))))

(event `Key|RightMouseButton`
  (params (Key :type "Key Structure"))
  (bind _pendulumref (`self.PendulumRef`))
  (bind _pendulumref_2 (`self.PendulumRef`))
  (bind _stringlength (`Pendulum.StringLength` _pendulumref))
  (bind _stringlength_2 (`Pendulum.StringLength` _pendulumref_2))
  (bind _rod (`Pendulum.Rod` _pendulumref_2))
  (bind (_relativescale3d_x _relativescale3d_y) (`KismetMathLibrary.BreakVector` (`SceneComponent.RelativeScale3D` _rod)))
  (:`Pressed`
    (bind _asthird_person_character (cast `/Game/ThirdPersonBP/Blueprints/ThirdPersonCharacter` (`GameplayStatics.GetPlayerCharacter` 0)))
    (bind _lengthincrement (`/Game/ThirdPersonBP/Blueprints/ThirdPersonCharacter.LengthIncrement` _asthird_person_character))
    (if (== _lengthincrement 1.0)
      (if (>= _stringlength_2 -90.0)
        (bind _output_get (set `Pendulum.StringLength` (+ _stringlength_2 -10.0) _pendulumref_2))
        (`SceneComponent.SetRelativeScale3D` _rod (`KismetMathLibrary.MakeVector` _relativescale3d_x _relativescale3d_y (* _stringlength_2 -0.01)) :!label _label_2)
        (`TextRenderComponent.K2_SetText` (`self.LengthValue`) (`KismetTextLibrary.Conv_DoubleToText` (* _output_get -0.01) "HalfToEven")))
      (elif (== _lengthincrement -1.0)
        (if (>= -60.0 _stringlength)
          (set `Pendulum.StringLength` (+ _stringlength 10.0) _pendulumref)
          (goto _label_2))))))

(fn `TurnOnOff`
  (params (Swtich :type "SceneComponent Object Reference") (SwitchOffset :type "Float (double-precision)"))
  (bind (_returnvalue_x _returnvalue_y _returnvalue_z) (`KismetMathLibrary.BreakVector` (`SceneComponent.K2_GetComponentLocation` Swtich)))
  (`SceneComponent.K2_SetWorldLocation` Swtich (`KismetMathLibrary.MakeVector` _returnvalue_x _returnvalue_y (+ _returnvalue_z SwitchOffset)) false false))

(fn `UserConstructionScript`)