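; Pendulum actor whose swing follows the ThirdPersonCharacter's IsSwitchOnForOscillation flag.
; Each tick it casts player character 0 and calls GeneralMotion with delta time while the flag is set, otherwise StopMotion.
; The construction script uses StringLength to offset the Ball vertically from PlaceHolder and to scale the Rod's Z to match.
; It enables input from player controller 0 on BeginPlay, though this graph binds no input events.
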(event `self.ReceiveBeginPlay`
  (`self.EnableInput` (`GameplayStatics.GetPlayerController` 0)))

(event `self.ReceiveTick`
  (params (DeltaSeconds :type "Float (single-precision)"))
  (bind _asthird_person_character (cast `/Game/ThirdPersonBP/Blueprints/ThirdPersonCharacter` (`GameplayStatics.GetPlayerCharacter` 0)))
  (if (`/Game/ThirdPersonBP/Blueprints/ThirdPersonCharacter.IsSwitchOnForOscillation` _asthird_person_character)
    (`self.GeneralMotion` DeltaSeconds)
    (else
      (`self.StopMotion`))))

(fn `UserConstructionScript`
  (bind _rod (`self.Rod`))
  (bind (_relativelocation_x _relativelocation_y _relativelocation_z) (`KismetMathLibrary.BreakVector` (`SceneComponent.RelativeLocation` (`self.PlaceHolder`))))
  (bind (_relativescale3d_x _relativescale3d_y) (`KismetMathLibrary.BreakVector` (`SceneComponent.RelativeScale3D` _rod)))
  (`SceneComponent.K2_SetRelativeLocation` (`self.Ball`) (`KismetMathLibrary.MakeVector` _relativelocation_x _relativelocation_y (+ _relativelocation_z (`self.StringLength`))) false false)
  (`SceneComponent.SetRelativeScale3D` _rod (`KismetMathLibrary.MakeVector` _relativescale3d_x _relativescale3d_y (* (`self.StringLength`) -0.01))))